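; BP_MazeManager builds a Pac-Man maze on a 100-unit grid, with helpers that turn row and column into world positions.
; Walls and a scaled background are static mesh components, while the ghost house, Pac-Man and ghosts are spawned actors.
; Pac-Man is possessed by player 0, and each ghost, chosen by type, receives references to the manager and Pac-Man.
; Ghost wall, dot and power pellet functions are stubs that create nothing.
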(fn `CreateGhostHouse`
  (params (row :type Integer) (collumn :type Integer))
  (returns (ReturnValue :type "Vector Structure"))
  (bind _returnvalue (`self.RowCollumn to Vector` row collumn))
  (`|SpawnActorFromClass` "/Game/Ghosts/GhostHouse.GhostHouse_C" (`KismetMathLibrary.Conv_VectorToTransform` _returnvalue) "Undefined" "OverrideRootScale" null null)
  (return _returnvalue))

(fn `CreateGhostWall`
  (params (row :type Integer) (collumn :type Integer))
  (returns (ReturnValue :type "Vector Structure"))
  (return (0.0 0.0 0.0)))

(fn `CreateMazeBackground`
  (bind _mazerows (`self.MazeRows`))
  (bind _mazecollumns (`self.MazeCollumns`))
  (`AddComponent|NODE_AddStaticMeshComponent-2` :`RelativeTransform` (`KismetMathLibrary.MakeTransform` (`KismetMathLibrary.MakeVector` (- (* _mazerows 50) 50.0) (+ (* _mazecollumns -50) 50.0) -100.0) (struct) (`KismetMathLibrary.MakeVector` (`KismetMathLibrary.Conv_IntToDouble` _mazerows) (`KismetMathLibrary.Conv_IntToDouble` _mazecollumns) 1.0)))
  (return))

(fn `CreatePacDot`
  (params (row :type Integer) (collumn :type Integer))
  (returns (ReturnValue :type "Vector Structure"))
  (return (`self.RowCollumn to Vector` row collumn)))

(fn `CreatePacWall`
  (params (row :type Integer) (collumn :type Integer))
  (returns (ReturnValue :type "Vector Structure"))
  (bind _returnvalue (`self.RowCollumn to Vector` row collumn))
  (bind _returnvalue_2 (`AddComponent|NODE_AddStaticMeshComponent-1` :`RelativeTransform` (`KismetMathLibrary.Conv_VectorToTransform` _returnvalue)))
  (`KismetArrayLibrary.Array_Add` (`self.Walls`) _returnvalue_2)
  (return _returnvalue))

(fn `CreatePowerPellet`
  (params (row :type Integer) (collumn :type Integer))
  (returns (ReturnValue :type "Vector Structure"))
  (return (`self.RowCollumn to Vector` row collumn)))

(fn `PlaceAGhost`
  (params (newGhostClass :type "EGhostType Enum" :default "Blinky") (spawnPlace :type "Vector Structure") (pacMan :type "PacMan Object Reference"))
  (returns (ReturnValue :type "GhostBase Object Reference"))
  (bind _asghost_base (castclass `GhostBase` (select `EGhostType` newGhostClass :`Blinky` "/Script/NeoPacMan3D.Blinky" :`Pinky` "/Script/NeoPacMan3D.Pinky" :`Inky` "/Script/NeoPacMan3D.Inky" :`Clyde` "/Script/NeoPacMan3D.Clyde" :!type "Object Class Reference")))
  (bind _returnvalue (`|SpawnActorFromClass` _asghost_base (`KismetMathLibrary.Conv_VectorToTransform` spawnPlace) "AlwaysSpawn" "OverrideRootScale" null self pacMan null))
  (return _returnvalue))

(fn `PlacePacMan`
  (params (row :type Integer) (collumn :type Integer))
  (returns (ReturnValue :type "PacMan Object Reference"))
  (bind _returnvalue (`|SpawnActorFromClass` "/Script/NeoPacMan3D.PacMan" (`KismetMathLibrary.Conv_VectorToTransform` (`self.RowCollumn to Vector` row collumn)) "AlwaysSpawn" "OverrideRootScale" null self null))
  (`Controller.Possess` (`GameplayStatics.GetPlayerController` 0) _returnvalue)
  (return _returnvalue))

(fn `UserConstructionScript`)