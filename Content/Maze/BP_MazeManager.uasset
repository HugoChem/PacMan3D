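; Maze manager for a Pac-Man game, providing spawn helpers for the maze, its pickups and its characters.
; Walls, pac-dots, power pellets and a background sized from row and column counts are static mesh actors built through CreateMeshActor.
; Pac-Man is spawned and possessed; ghosts spawn by selected type with manager and Pac-Man references.
; CreateGhostWall is empty, and both ghost house helpers spawn BigGhostHouse, differing only in offset.
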(fn `CreateBigGhostHouse`
  (params (pos :type "Vector Structure (by ref)"))
  (`|SpawnActorFromClass` "/Game/Maze/BigGhostHouse.BigGhostHouse_C" (`KismetMathLibrary.Conv_VectorToTransform` (+ pos (0.0 -50.0 0.0))) "Undefined" "OverrideRootScale" null null)
  (return))

(fn `CreateGhostWall`
  (params (pos :type "Vector Structure (by ref)"))
  (returns (ReturnValue :type "StaticMeshActor Object Reference"))
  (return null))

(fn `CreateLittleGhostHouse`
  (params (pos :type "Vector Structure (by ref)"))
  (`|SpawnActorFromClass` "/Game/Maze/BigGhostHouse.BigGhostHouse_C" (`KismetMathLibrary.Conv_VectorToTransform` pos) "Undefined" "OverrideRootScale" null null)
  (return))

(fn `CreateMazeBackground`
  (bind _mazerows (`self.MazeRows`))
  (bind _mazecollumns (`self.MazeCollumns`))
  (`self.CreateMeshActor` (`KismetMathLibrary.MakeTransform` (`KismetMathLibrary.MakeVector` (- (* _mazerows 50) 50.0) (+ (* _mazecollumns -50) 50.0) -100.0) (struct) (`KismetMathLibrary.MakeVector` (`KismetMathLibrary.Conv_IntToDouble` _mazerows) (`KismetMathLibrary.Conv_IntToDouble` _mazecollumns) 1.0)) "/Engine/VREditor/BasicMeshes/SM_Cube_02.SM_Cube_02" "/Engine/VREditor/BasicMeshes/MI_Cube_02.MI_Cube_02")
  (return))

(fn `CreateMeshActor`
  (params (SpawnTransform :type "Transform Structure") (Mesh :type "StaticMesh Object Reference") (Material :type "MaterialInterface Object Reference"))
  (returns (OutputPin :type "StaticMeshActor Object Reference"))
  (bind _returnvalue (`|SpawnActorFromClass` "/Script/Engine.StaticMeshActor" SpawnTransform "Undefined" "OverrideRootScale" null null))
  (bind _staticmeshcomponent (`StaticMeshActor.StaticMeshComponent` _returnvalue))
  (`StaticMeshComponent.SetStaticMesh` _staticmeshcomponent (`local.Mesh`))
  (`PrimitiveComponent.SetMaterial` _staticmeshcomponent 0 (`local.Material`))
  (return _returnvalue))

(fn `CreatePacDot`
  (params (pos :type "Vector Structure (by ref)"))
  (returns (ReturnValue :type "StaticMeshActor Object Reference"))
  (bind _outputpin (`self.CreateMeshActor` (`KismetMathLibrary.MakeTransform` pos (struct) (0.3 0.3 0.3)) "/Engine/BasicShapes/Sphere.Sphere" "/Game/Maze/MI_PacDot.MI_PacDot"))
  (return _outputpin))

(fn `CreatePacWall`
  (params (pos :type "Vector Structure (by ref)"))
  (returns (ReturnValue :type "StaticMeshActor Object Reference"))
  (bind _outputpin (`self.CreateMeshActor` (`KismetMathLibrary.Conv_VectorToTransform` pos) "/Engine/VREditor/BasicMeshes/SM_Cube_02.SM_Cube_02" "/Engine/VREditor/BasicMeshes/MI_Cube_02.MI_Cube_02"))
  (`StaticMeshActor.SetMobility` _outputpin "Movable")
  (return _outputpin))

(fn `CreatePowerPellet`
  (params (pos :type "Vector Structure (by ref)"))
  (returns (ReturnValue :type "StaticMeshActor Object Reference"))
  (bind _outputpin (`self.CreateMeshActor` (`KismetMathLibrary.MakeTransform` pos (struct) (0.5 0.5 0.5)) "/Engine/BasicShapes/Sphere.Sphere" "/Game/Maze/MI_PowerPellet.MI_PowerPellet"))
  (return _outputpin))

(fn `PlaceAGhost`
  (params (newGhostClass :type "EGhostType Enum" :default "Blinky") (pos :type "Vector Structure (by ref)") (pacMan :type "PacMan Object Reference"))
  (returns (ReturnValue :type "GhostBase Object Reference"))
  (bind _asghost_base (castclass `GhostBase` (select `EGhostType` newGhostClass :`Blinky` "/Script/NeoPacMan3D.Blinky" :`Pinky` "/Script/NeoPacMan3D.Pinky" :`Inky` "/Script/NeoPacMan3D.Inky" :`Clyde` "/Script/NeoPacMan3D.Clyde" :!type "Object Class Reference")))
  (bind _returnvalue (`|SpawnActorFromClass` _asghost_base (`KismetMathLibrary.Conv_VectorToTransform` pos) "AlwaysSpawn" "OverrideRootScale" null self pacMan null))
  (return _returnvalue))

(fn `PlacePacMan`
  (params (pos :type "Vector Structure (by ref)") (offset :type Boolean))
  (returns (ReturnValue :type "PacMan Object Reference"))
  (bind _returnvalue (`|SpawnActorFromClass` "/Game/PacMan/BP_PacMan.BP_PacMan_C" (`KismetMathLibrary.Conv_VectorToTransform` (`KismetMathLibrary.SelectVector` (+ pos (0.0 -50.0 0.0)) pos offset)) "AlwaysSpawn" "OverrideRootScale" null self null))
  (`Controller.Possess` (`GameplayStatics.GetPlayerController` 0) _returnvalue)
  (set `PacMan.TileProgress` (select `bool` offset :`true` 0.5 :!type "Float (single-precision)") _returnvalue)
  (return _returnvalue))

(fn `UserConstructionScript`)